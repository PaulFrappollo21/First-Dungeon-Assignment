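; Proximity sliding door Blueprint that MyCharacter opens with E while inside its Box trigger, unless IsLocked is set.
; Box overlap toggles input; the MoveDoor timeline moves DoorMesh and reverses when the character leaves.
; The construction script colors DoorLight red or green by lock state.
; TurnonorOff sets IsOn, which makes Tick clear IsLocked every frame and turn the light green, leaving its red branch unreachable.
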(event OnComponentBeginOverlap(Box)
  (params (OverlappedComponent :type Primitive%20Component%20Object%20Reference) (OtherActor :type Actor%20Object%20Reference) (OtherComp :type Primitive%20Component%20Object%20Reference) (OtherBodyIndex :type Integer) (bFromSweep :type Boolean) (SweepResult :type Hit%20Result%20Structure%20%28by%20ref%29))
  (Utilities|Casting|CastToMyCharacter OtherActor)
  (Input|EnableInput (Game|GetPlayerController 0)))

(event OnComponentEndOverlap(Box)
  (params (OverlappedComponent :type Primitive%20Component%20Object%20Reference) (OtherActor :type Actor%20Object%20Reference) (OtherComp :type Primitive%20Component%20Object%20Reference) (OtherBodyIndex :type Integer))
  (Utilities|Casting|CastToMyCharacter OtherActor)
  (Input|DisableInput (Game|GetPlayerController 0))
  (bind _moving_door (Timeline|Move%20Door Reverse)
    (:Update
      (Transformation|SetRelativeLocation (Variables|Default|GetDoor%20Mesh) _moving_door false false))))

(event EventTurnonorOff
  (params (OnOrOff :type Boolean))
  (Variables|Default|SetIsOn OnOrOff))

(event EventTick
  (params (DeltaSeconds :type Float%20%28single-precision%29))
  (bind _door_light (Variables|Default|GetDoor%20Light))
  (if (Variables|Default|GetIsOn)
    (bind _output_get (Variables|Default|SetIsLocked false))
    (if _output_get
      (Rendering|Components|Light|SetLightColor _door_light "(R=1.000000,G=0.032916,B=0.000000,A=1.000000)" true)
      (else
        (Rendering|Components|Light|SetLightColor _door_light "(R=0.026313,G=1.000000,B=0.000000,A=1.000000)" true)))))

(event Input|KeyboardEvents|E
  (params (Key :type Key%20Structure))
  (:Pressed
    (if (not (Variables|Default|GetIsLocked))
      (bind _moving_door (Timeline|Move%20Door Play)
        (:Update
          (Transformation|SetRelativeLocation (Variables|Default|GetDoor%20Mesh) _moving_door false false))))))

(fn ConstructionScript
  (bind _door_light (Variables|Default|GetDoor%20Light))
  (if (Variables|Default|GetIsLocked)
    (Rendering|Components|Light|SetLightColor _door_light "(R=1.000000,G=0.032916,B=0.000000,A=1.000000)" true)
    (else
      (Rendering|Components|Light|SetLightColor _door_light "(R=0.026313,G=1.000000,B=0.000000,A=1.000000)" true))))