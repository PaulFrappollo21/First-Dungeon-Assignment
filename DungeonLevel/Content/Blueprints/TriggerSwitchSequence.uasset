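; Trigger switch that, while active, lets the interact input turn on its TargetActor when pressed during an overlap.
; A gate opened and closed by actor overlap filters the input, and a successful press switches the sphere to its SwitchOn material.
; TurnonorOff sets the active state, resets the sphere to black either way, and sends the target an off message when deactivated.
; BeginPlay applies the initial state.
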(event Collision|EventActorBeginOverlap
  (params (OtherActor :type Actor%20Object%20Reference))
  (Utilities|FlowControl|Gate true) ; enters at Open
)

(event Collision|EventActorEndOverlap
  (params (OtherActor :type Actor%20Object%20Reference))
  (Utilities|FlowControl|Gate true) ; enters at Close
)

(event EventTurnonorOff
  (params (OnOrOff :type Boolean))
  (bind _sphere (Variables|Default|GetSphere))
  (bind _output_get (Variables|Default|SetisActive OnOrOff))
  (if _output_get
    (Rendering|Material|SetMaterial _sphere 0 "/Game/Materials/BlackColor.BlackColor")
    (else
      (Rendering|Material|SetMaterial _sphere 0 "/Game/Materials/BlackColor.BlackColor")
      (Class|BPInterface|TurnonorOff(Message) (Variables|Default|GettargetActor) false))))

(event EventBeginPlay
  (CallFunction|TurnonorOff (Variables|Default|GetisActive)))

(event Input|ActionEvents|InputActioninteract
  (params (Key :type Key%20Structure))
  (:Pressed
    (if (Variables|Default|GetisActive)
      (Utilities|FlowControl|Gate true
        (:Exit
          (Class|BPInterface|TurnonorOff(Message) (Variables|Default|GettargetActor) true)
          (Rendering|Material|SetMaterial (Variables|Default|GetSphere) 0 "/Game/Materials/SwitchOn.SwitchOn"))))))

(fn ConstructionScript)