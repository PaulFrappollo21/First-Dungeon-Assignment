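; A switchable rotating block actor that spins its Cube component while turned on.
; Tick adds local yaw scaled by RotationSpeed and delta time, keeping the spin frame-rate independent, whenever IsOn is true.
; The TurnonorOff event sets IsOn from its OnOrOff input, so the rotation can be started or stopped.
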(event EventBeginPlay)

(event Collision|EventActorBeginOverlap
  (params (OtherActor :type Actor%20Object%20Reference)))

(event EventTick
  (params (DeltaSeconds :type Float%20%28single-precision%29))
  (Variables|Default|SetDeltaSeconds DeltaSeconds)
  (if (Variables|Default|GetIsOn)
    (Transformation|AddLocalRotation (Variables|Default|GetCube) (Math|Rotator|MakeRotator 0.0 0.0 (* (Variables|Default|GetRotationSpeed) (Variables|Default|GetDeltaSeconds))) false false)))

(event EventTurnonorOff
  (params (OnOrOff :type Boolean))
  (Variables|Default|SetIsOn OnOrOff))

(fn ConstructionScript)