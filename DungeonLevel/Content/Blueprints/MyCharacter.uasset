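; Player character Blueprint handling movement, look, jump, pause, projectile firing and physics object pickup.
; Right mouse line-traces from the camera for physics bodies and grabs the hit through a PhysicsHandle, whose target follows GrabLocation each Tick.
; Drop on release is empty, and both branches of the pause FlipFlop pause the game.
; Fire spawns MyProjectile at a raised, rightward offset along control rotation.
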(event Custom|Pick%20Up
  (bind _camera (Variables|Default|GetCamera))
  (bind _returnvalue (Transformation|GetWorldLocation _camera))
  (bind _outhit (Collision|LineTraceForObjects _returnvalue (+ _returnvalue (* (Math|Vector|GetForwardVector _camera) 1e+04)) (Utilities|Array|MakeArray "ObjectTypeQuery4") false (Utilities|Array|MakeArray (stale _asmy_character)) "ForOneFrame"))
  (if true
    (Class|PhysicsHandleComponent|GrabComponentatLocation (Variables|Default|GetPhysicsHandle) (.HitComponent (Collision|BreakHitResult _outhit)) "None" (.Location (Collision|BreakHitResult _outhit)))))

(event Custom|Drop)

(event EventTick
  (params (DeltaSeconds :type Float%20%28single-precision%29))
  (Physics|Components|PhysicsHandle|SetTargetLocation (Variables|Default|GetPhysicsHandle) (Transformation|GetWorldLocation (Variables|Default|GetGrab%20Location))))

(event Input|ActionEvents|InputActionJump
  (params (Key :type Key%20Structure))
  ;[1 1 1] Enable Player Pause and Jump
  (:Pressed
    (Character|Jump)))

(event Input|ActionEvents|InputActionPause
  (params (Key :type Key%20Structure))
  ;[1 1 1] Enable Player Pause and Jump
  (:Pressed
    (Utilities|FlowControl|FlipFlop
      (:A
        (Game|SetGamePaused true))
      (:B
        (Game|SetGamePaused true)))))

(event Input|ActionEvents|InputActionFire
  (params (Key :type Key%20Structure))
  ;[1 1 1] Fire Projectile
  (:Pressed
    (Game|SpawnActorfromClass "/Game/Blueprints/MyProjectile.MyProjectile_C" (Math|Transform|MakeTransform (+ (+ (.location (Transformation|GetActorTransform)) "0, 0,50.000000") (* (Transformation|GetActorRightVector) 75.0)) (Pawn|GetControlRotation :!class /Script/Engine.Pawn) "1,1,1") "Undefined" 0 0)))

(event Input|AxisEvents|InputAxisWalk
  (params (AxisValue :type Float%20%28single-precision%29))
  ;[1 1 1] Player Movement
  (Pawn|Input|AddMovementInput (Transformation|GetActorForwardVector) AxisValue false))

(event Input|AxisEvents|InputAxisStrafe
  (params (AxisValue :type Float%20%28single-precision%29))
  ;[1 1 1] Player Movement
  (Pawn|Input|AddMovementInput (Transformation|GetActorRightVector) AxisValue false))

(event Input|AxisEvents|InputAxisLookV
  (params (AxisValue :type Float%20%28single-precision%29))
  ;[1 1 1] Comment
  (Pawn|Input|AddControllerPitchInput AxisValue))

(event Input|AxisEvents|InputAxisLookH
  (params (AxisValue :type Float%20%28single-precision%29))
  ;[1 1 1] Comment
  (Pawn|Input|AddControllerYawInput AxisValue))

(event Input|MouseEvents|RightMouseButton
  (params (Key :type Key%20Structure))
  (:Pressed
    (CallFunction|PickUp))
  (:Released
    (CallFunction|Drop)))

(fn ConstructionScript)