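; Conveyor belt actor that pushes any actor overlapping its box along the belt's forward direction.
; Each tick it offsets those actors without sweep by the mesh's forward vector times Speed and delta time.
; The construction script creates a dynamic material on the mesh to set the color, arrow scale and scroll speed.
; The visual track speed is a separate variable from the movement speed.
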(event EventBeginPlay)

(event Collision|EventActorBeginOverlap
  (params (OtherActor :type Actor%20Object%20Reference)))

(event EventTick
  (params (DeltaSeconds :type Float%20%28single-precision%29))
  (for _array_element (Collision|GetOverlappingActors (Variables|Default|GetBox) 0 :!class /Script/Engine.PrimitiveComponent)
    ;[1 1 1] Moves Things
    (Transformation|AddActorWorldOffset _array_element (* (Math|Vector|GetForwardVector (Transformation|GetWorldRotation (Variables|Default|GetStaticMesh))) (* DeltaSeconds (Variables|Default|GetSpeed))))))

(fn ConstructionScript
  (bind _staticmesh (Variables|Default|GetStaticMesh))
  (bind _returnvalue (Rendering|Material|CreateDynamicMaterialInstance _staticmesh 0 0 "None" :!class /Script/Engine.PrimitiveComponent))
  (Rendering|Material|SetMaterial _staticmesh 0 _returnvalue)
  (Rendering|Material|SetVectorParameterValue _returnvalue "Color" (Variables|Default|GetColor) :!class /Script/Engine.MaterialInstanceDynamic)
  (Rendering|Material|SetScalarParameterValue _returnvalue "X_Scale" (Variables|Default|GetArrowScales) :!class /Script/Engine.MaterialInstanceDynamic)
  (Rendering|Material|SetScalarParameterValue _returnvalue "X_Speed" (Variables|Default|GetTrackSpeed) :!class /Script/Engine.MaterialInstanceDynamic))