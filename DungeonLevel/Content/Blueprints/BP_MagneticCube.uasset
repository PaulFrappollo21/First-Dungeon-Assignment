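; BP_MagneticCube is a cube actor whose magnetic polarity is set by the fluid it touches.
; On begin overlap, it checks whether the other actor's class is exactly BP_NegFluid or BP_PosFluid.
; A match swaps the cube's material to that fluid's material and sets the IsPositive flag to false or true accordingly.
; The file holds no attraction or repulsion logic, only this polarity state and its visual.
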(event EventBeginPlay)

(event Collision|EventActorBeginOverlap
  (params (OtherActor :type Actor%20Object%20Reference))
  (bind _returnvalue (Utilities|GetClass OtherActor))
  (if (== _returnvalue "/Game/Blueprints/BP_NegFluid.BP_NegFluid_C")
    (Rendering|Material|SetMaterial (Variables|Default|GetCube) 0 "/Game/Materials/NegFluidMat.NegFluidMat")
    (Variables|Default|SetIsPositive false)
    (elif (== _returnvalue "/Game/Blueprints/BP_PosFLuid.BP_PosFluid_C")
      (Rendering|Material|SetMaterial (Variables|Default|GetCube) 0 "/Game/Materials/PosFluidMat.PosFluidMat")
      (Variables|Default|SetIsPositive true))))

(event EventTick
  (params (DeltaSeconds :type Float%20%28single-precision%29)))

(fn ConstructionScript)